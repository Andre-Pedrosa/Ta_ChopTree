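; BP_branch is an interactable tree whose branches the player cuts by pressing C.
; Its Capsule detects components named "TreeChopBox" by display-name substring, then enables input and shows a WG_PressC prompt in Portuguese.
; Ending the overlap disables input and removes the prompt.
; Pressing C calls RemoveBranch, which spawns BP_TreeCut at the Tree component's transform and destroys this actor.
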(event OnComponentBeginOverlap(Capsule)
  (params (OverlappedComponent :type Primitive%20Component%20Object%20Reference) (OtherActor :type Actor%20Object%20Reference) (OtherComp :type Primitive%20Component%20Object%20Reference) (OtherBodyIndex :type Integer) (bFromSweep :type Boolean) (SweepResult :type Hit%20Result%20Structure%20%28by%20ref%29))
  (if (Utilities|String|Contains (Utilities|GetDisplayName OtherComp) "TreeChopBox")
    (Development|PrintString "Branch overlap")
    (Input|EnableInput (Game|GetPlayerController 0))
    (bind _returnvalue (UserInterface|CreateWidget "/Game/WG_PressC.WG_PressC_C"))
    (Rendering|Components|TextRender|SetText (Variables|/Game/WG_PressC.WG_PressC_C|GetText _returnvalue) "Pressione 'C' para cortar os ramos da árvore")
    (UserInterface|Viewport|AddtoViewport _returnvalue 0)))

(event OnComponentEndOverlap(Capsule)
  (params (OverlappedComponent :type Primitive%20Component%20Object%20Reference) (OtherActor :type Actor%20Object%20Reference) (OtherComp :type Primitive%20Component%20Object%20Reference) (OtherBodyIndex :type Integer))
  (if (Utilities|String|Contains (Utilities|GetDisplayName OtherComp) "TreeChopBox")
    (Input|DisableInput (Game|GetPlayerController 0))
    (Widget|RemovefromParent (stale OnComponentBeginOverlap(Capsule) _returnvalue))))

(event EventBeginPlay)

(event Collision|EventActorBeginOverlap
  (params (OtherActor :type Actor%20Object%20Reference)))

(event EventTick
  (params (DeltaSeconds :type Float%20%28single-precision%29)))

(event Input|KeyboardEvents|C
  (params (Key :type Key%20Structure :default "None"))
  (:Pressed
    (CallFunction|RemoveBranch)))

(fn ConstructionScript)

(fn RemoveBranch
  (Game|SpawnActorfromClass "/Game/BP_TreeCut.BP_TreeCut_C" (Transformation|GetWorldTransform (Variables|Default|GetTree)) "AlwaysSpawn" 0 0)
  (Actor|DestroyActor))