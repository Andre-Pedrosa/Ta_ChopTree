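; Choppable tree actor that copies its static mesh to a procedural mesh, or takes one from the character.
; Overlap with a "Plane" component enables input; two left clicks slice at Cut1 then Cut2, adding wood caps, physics and impulses.
; UpdateBorders nudges Top and Bottom markers inward until they overlap the mesh, then prints the length.
; An older path slicing at the character's plane and respawning the actor is disconnected.
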(event OnComponentBeginOverlap(ProceduralMesh)
  (params (OverlappedComponent :type Primitive%20Component%20Object%20Reference) (OtherActor :type Actor%20Object%20Reference) (OtherComp :type Primitive%20Component%20Object%20Reference) (OtherBodyIndex :type Integer) (bFromSweep :type Boolean) (SweepResult :type Hit%20Result%20Structure%20%28by%20ref%29))
  (if (Utilities|String|Contains (Utilities|GetDisplayName OtherComp) "Plane")
    (Development|PrintString "Enable Input" true true "(R=0.000000,G=1.000000,B=0.000000,A=1.000000)" 5.0)
    (Input|EnableInput (Game|GetPlayerController 0))))

(event OnComponentEndOverlap(ProceduralMesh)
  (params (OverlappedComponent :type Primitive%20Component%20Object%20Reference) (OtherActor :type Actor%20Object%20Reference) (OtherComp :type Primitive%20Component%20Object%20Reference) (OtherBodyIndex :type Integer))
  (if (Utilities|String|Contains (Utilities|GetDisplayName OtherComp) "Plane")
    (Development|PrintString "Disable Input" true true "(R=0.094573,G=1.000000,B=0.000000,A=1.000000)" 5.0)
    (Input|DisableInput (Game|GetPlayerController 0))))

(event Custom|Timer
  (bind _returnvalue (Utilities|Time|SetTimerbyFunctionName 0 "UpdateBorders" 0.1 true)))

(event Custom|StopTimer
  (Utilities|Time|ClearandInvalidateTimerbyHandle (stale Custom|Timer _returnvalue)))

(event EventBeginPlay)

(event Collision|EventActorBeginOverlap
  (params (OtherActor :type Actor%20Object%20Reference)))

(event EventTick
  (params (DeltaSeconds :type Float%20%28single-precision%29)))

(event Input|MouseEvents|LeftMouseButton
  (params (Key :type Key%20Structure :default "None"))
  (bind _cut2 (Variables|Default|Getcut2))
  (bind _cutcount (Variables|Default|GetCutCount))
  (bind _cut1 (Variables|Default|Getcut1))
  (bind _returnvalue (Transformation|GetWorldLocation _cut2))
  (bind _returnvalue_2 (Transformation|GetWorldLocation _cut1))
  (:Pressed
    (if (== _cutcount 0)
      (bind _outotherhalfprocmesh (Class|KismetProceduralMeshLibrary|SliceProceduralMesh (Variables|Default|GetProceduralMesh) _returnvalue_2 (Math|Vector|GetUpVector _cut1) true "CreateNewSectionForCap" "/Game/StarterContent/Materials/M_Wood_Walnut.M_Wood_Walnut"))
      (Physics|SetSimulatePhysics _outotherhalfprocmesh true)
      (Physics|AddRadialImpulse _outotherhalfprocmesh _returnvalue_2 3e+02 2e+02 "RIF_Constant" true)
      (Math|Integer|IncrementInt (Variables|Default|GetCutCount) :!label _label)
      (elif (== 1 _cutcount)
        (bind _outotherhalfprocmesh_2 (Class|KismetProceduralMeshLibrary|SliceProceduralMesh (Variables|Default|GetProceduralMesh) _returnvalue (Math|Vector|GetUpVector _cut2) true "CreateNewSectionForCap" "/Game/StarterContent/Materials/M_Wood_Walnut.M_Wood_Walnut"))
        (Physics|SetSimulatePhysics _outotherhalfprocmesh_2 true)
        (Physics|AddRadialImpulse _outotherhalfprocmesh_2 _returnvalue 3e+02 2e+02 "RIF_Constant" true)
        (goto _label)))))

(fn ConstructionScript
  (bind _outactors (Actor|GetAllActorsOfClass "/Game/ThirdPersonBP/Blueprints/ThirdPersonCharacter.ThirdPersonCharacter_C"))
  (if (Variables|/Game/ThirdPersonBP/Blueprints/ThirdPersonCharacter.ThirdPersonCharacter_C|GetProceduralBool (Utilities|Array|Get(acopy) _outactors))
    (Variables|Default|SetProceduralMesh (Variables|/Game/ThirdPersonBP/Blueprints/ThirdPersonCharacter.ThirdPersonCharacter_C|GetProcedural (Utilities|Array|Get(acopy) _outactors)))
    (Variables|/Game/ThirdPersonBP/Blueprints/ThirdPersonCharacter.ThirdPersonCharacter_C|SetProceduralBool (Utilities|Array|Get(acopy) _outactors) false)
    (else
      (Class|KismetProceduralMeshLibrary|CopyProceduralMeshfromStaticMeshComponent (Variables|Default|GetStaticMesh) 0 (Variables|Default|GetProceduralMesh) true)
      (Variables|Default|Setname (Utilities|String|StringToName (Utilities|GetDisplayName (Variables|Default|GetProceduralMesh))))))
  (CallFunction|GetLenght))

(fn UpdateBorders
  (bind _bottom (Variables|Default|Getbottom))
  (bind _top (Variables|Default|Gettop))
  (bind _output_get (Variables|Default|SetLoop true))
  (while _output_get
    (Variables|Default|SetBottomInPlace false)
    (Variables|Default|SetTopInPlace false)
    (for _array_element (Class|PrimitiveComponent|GetOverlappingComponents (Variables|Default|Getbottom))
      (if (Utilities|Enum|Equal(Enum) (Utilities|GetDisplayName _array_element) (Utilities|String|ToString(Name) (Variables|Default|Getname)))
        (Variables|Default|SetBottomInPlace true)))
    (if (Variables|Default|GetBottomInPlace)
      _
      (else
        (Transformation|SetRelativeLocation _bottom (+ "0, 0,1.000000" (Variables|/Script/Engine.SceneComponent|GetRelativeLocation _bottom)) false false)))
    (for _array_element_2 (Class|PrimitiveComponent|GetOverlappingComponents (Variables|Default|Gettop))
      (if (Utilities|Enum|Equal(Enum) (Utilities|GetDisplayName _array_element_2) (Utilities|String|ToString(Name) (Variables|Default|Getname)))
        (Variables|Default|SetTopInPlace true)))
    (if (Variables|Default|GetTopInPlace)
      _
      (else
        (Transformation|SetRelativeLocation _top (+ (Variables|/Script/Engine.SceneComponent|GetRelativeLocation _top) "0, 0,-1.000000") false false)))
    (if (and (Variables|Default|GetTopInPlace) (Variables|Default|GetBottomInPlace))
      (CallFunction|GetLenght)
      (Variables|Default|SetLoop false))))

(fn GetLenght
  (Development|PrintString (Utilities|String|ToString(Float) (- (.z (Variables|/Script/Engine.SceneComponent|GetRelativeLocation (Variables|Default|Gettop))) (.z (Variables|/Script/Engine.SceneComponent|GetRelativeLocation (Variables|Default|Getbottom)))))))