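; BP_tree is a choppable tree that the player cuts down with the C key.
; Overlap with a component named TreeChopBox enables input and shows a WG_PressC prompt, both removed on end overlap.
; Each press updates the widget and, after a short delay, reduces health by a fixed amount.
; At zero health, the tree component is destroyed, a replacement mesh is added and a BP_branch spawns with slightly randomized rotation.
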(event OnComponentBeginOverlap(Tree)
  (params (OverlappedComponent :type Primitive%20Component%20Object%20Reference) (OtherActor :type Actor%20Object%20Reference) (OtherComp :type Primitive%20Component%20Object%20Reference) (OtherBodyIndex :type Integer) (bFromSweep :type Boolean) (SweepResult :type Hit%20Result%20Structure%20%28by%20ref%29))
  (if (Utilities|String|Contains (Utilities|GetDisplayName OtherComp) "TreeChopBox")
    (Development|PrintString "TreeChopBox Begin Overlap")
    (Input|EnableInput (Game|GetPlayerController 0))
    (bind _returnvalue (UserInterface|CreateWidget "/Game/WG_PressC.WG_PressC_C"))
    (Rendering|Components|TextRender|SetText (Variables|/Game/WG_PressC.WG_PressC_C|GetText _returnvalue) "Pressione 'C' para cortar a árvore")
    (UserInterface|Viewport|AddtoViewport _returnvalue 0)))

(event OnComponentEndOverlap(Tree)
  (params (OverlappedComponent :type Primitive%20Component%20Object%20Reference) (OtherActor :type Actor%20Object%20Reference) (OtherComp :type Primitive%20Component%20Object%20Reference) (OtherBodyIndex :type Integer))
  (if (Utilities|String|Contains (Utilities|GetDisplayName OtherComp) "TreeChopBox")
    (Development|PrintString "TreeChopBox End Overlap")
    (Input|DisableInput (Game|GetPlayerController 0))
    (Widget|RemovefromParent (stale OnComponentBeginOverlap(Tree) _returnvalue))))

(event EventBeginPlay)

(event Collision|EventActorBeginOverlap
  (params (OtherActor :type Actor%20Object%20Reference)))

(event EventTick
  (params (DeltaSeconds :type Float%20%28single-precision%29)))

(event Input|KeyboardEvents|C
  (params (Key :type Key%20Structure :default "None"))
  (:Pressed
    (Utilities|Casting|CastToThirdPersonCharacter (Utilities|Array|Get(acopy) (Collision|GetOverlappingActors "/Game/ThirdPersonBP/Blueprints/ThirdPersonCharacter.ThirdPersonCharacter_C" :!class /Script/Engine.Actor)))))

(event Input|KeyboardEvents|C
  (params (Key :type Key%20Structure :default "None"))
  (:Pressed
    (Variables|/Game/WG_PressC.WG_PressC_C|SetIsPressed (stale OnComponentBeginOverlap(Tree) _returnvalue) true)
    (Utilities|FlowControl|Delay 0.2)
    (CallFunction|TakeDamage))
  (:Released
    (Variables|/Game/WG_PressC.WG_PressC_C|SetIsPressed (stale OnComponentBeginOverlap(Tree) _returnvalue) false)))

(fn ConstructionScript)

(fn TakeDamage
  (bind _output_get (Variables|Default|SetHealthh (- (Variables|Default|GetHealthh) 25)))
  (if (== _output_get 0)
    (Components|DestroyComponent (Variables|Default|GetTree))
    (CallFunction|ReplaceMesh)))

(fn ReplaceMesh
  (bind _defaultsceneroot (Variables|Default|GetDefaultSceneRoot))
  (AddComponent|AddStaticMeshComponent false)
  (Game|SpawnActorfromClass "/Game/BP_branch.BP_branch_C" (Math|Transform|MakeTransform (Transformation|GetWorldLocation _defaultsceneroot) (Math|Conversions|RotationFromXVector (+ (Math|Rotator|GetRotationXVector (Transformation|GetWorldRotation _defaultsceneroot)) (Math|Conversions|ToVector(Float) (Math|Random|RandomFloatinRange 0.05 0.1)))) "1,1,1") "AlwaysSpawn" 0 0))